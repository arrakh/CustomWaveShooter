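; BP_EnemyProjectile is an enemy projectile that damages the player on contact and destroys itself after a short lifetime.
; The construction script applies ProjectileSpeed to the movement component's initial and max speed.
; On overlap with the player's tagged capsule, it calls Hit with Knockback, plays a hurt camera shake and destroys itself.
; Hit receives the sphere location saved at BeginPlay as the damager location, rather than the impact point.
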(event `Destroy`
  (`self.K2_DestroyActor`))

(event `self.ReceiveBeginPlay`
  (`KismetSystemLibrary.K2_SetTimerDelegate` (delegate `Destroy`) 3.0)
  (set `self.InitVector` (`SceneComponent.K2_GetComponentLocation` (`self.Sphere`))))

(event `self.Sphere.OnComponentBeginOverlap`
  (params (OverlappedComponent :type "PrimitiveComponent Object Reference") (OtherActor :type "Actor Object Reference") (OtherComp :type "PrimitiveComponent Object Reference") (OtherBodyIndex :type Integer) (bFromSweep :type Boolean) (SweepResult :type "HitResult Structure (by ref)"))
  (bind _asbp_player (cast `/Game/Blueprints/BP_Player` OtherActor))
  (if (`ActorComponent.ComponentHasTag` OtherComp "PlayerCapsule")
    (`/Game/Blueprints/BP_Player.Hit` _asbp_player (`self.InitVector`) (`self.Knockback`))
    (`GameplayStatics.PlayWorldCameraShake` "/Game/Blueprints/BP_HurtShake.BP_HurtShake_C" (`SceneComponent.K2_GetComponentLocation` (`Character.CapsuleComponent` _asbp_player)) 0.0 99999.0)
    (`self.K2_DestroyActor`)))

(fn `UserConstructionScript`
  (bind _projectilemovement (`self.ProjectileMovement`))
  (bind _projectilespeed (`self.ProjectileSpeed`))
  (set `ProjectileMovementComponent.MaxSpeed` _projectilespeed _projectilemovement)
  (set `ProjectileMovementComponent.InitialSpeed` _projectilespeed _projectilemovement))