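; Base enemy character with a directional flipbook sprite that pursues the player, shoots projectiles and self-destructs on contact, applying knockback.
; Looping timers replace Tick to copy the player sprite's rotation, update aim and range checks, pick walk or idle flipbooks, and fire.
; Pawn sensing starts AI movement toward the player and halts it inside the detection radius.
; Damage launches it backward, and death awards score and coins with explosion and camera shake.
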(event `BetterTick`
  (bind (_returnvalue_x _returnvalue_y) (`KismetMathLibrary.BreakVector` (`self.GetActorForwardVector`)))
  (bind _returnvalue (`self.GetDistanceTo` (`self.PlayerRef`)))
  (bind _sprite (`PaperCharacter.Sprite` (`self.PlayerRef`)))
  (`SceneComponent.K2_SetWorldRotation` (`self.Sprite`) (`SceneComponent.K2_GetComponentRotation` _sprite) false false)
  (set `self.DirectionVector` (`KismetMathLibrary.MakeVector2D` _returnvalue_x _returnvalue_y))
  (set `self.AimAngle` (`KismetMathLibrary.FindLookAtRotation` (`SceneComponent.K2_GetComponentLocation` (`self.CapsuleComponent`)) (`SceneComponent.K2_GetComponentLocation` _sprite)))
  (set `self.isPlayerInRange` (<= _returnvalue (`self.DetectRadius`)))
  (set `self.isInShootingRange` (<= _returnvalue (`self.ShootRadius`))))

(event `self.ReceiveBeginPlay`
  ;[1 1 1] Begin
  (bind _outactors (`GameplayStatics.GetAllActorsOfClass` "/Game/Blueprints/BP_Player.BP_Player_C"))
  (set `self.PlayerRef` (`|GetArrayItem` _outactors))
  (bind _outactors_2 (`GameplayStatics.GetAllActorsOfClass` "/Game/Blueprints/BP_GameModeBase.BP_GameModeBase_C"))
  (set `self.GM` (`|GetArrayItem` _outactors_2))
  (`KismetSystemLibrary.K2_SetTimerDelegate` (delegate `BetterTick`) 0.01 true)
  (`KismetSystemLibrary.K2_SetTimer` null "SetSprite" 0.01 true)
  (`KismetSystemLibrary.K2_SetTimer` null "Fire" (`self.FireRate`) true)
  (set `CharacterMovementComponent.MaxWalkSpeed` (`self.WalkSpeed`) (`self.CharacterMovement`)))

(event `self.PawnSensing.OnSeePawn`
  (params (Pawn :type "Pawn Object Reference"))
  (if (`self.isPlayerInRange`)
    (`NavMovementComponent.StopActiveMovement` (`self.CharacterMovement`))
    (goto _label :!via `Reset`)
    (else
      (`/Engine/EditorBlueprintResources/StandardMacros.DoOnce` false :!label _label
        (:`Completed`
          (bind _asbp_player (cast `/Game/Blueprints/BP_Player` Pawn))
          (`|AIMoveTo` self (0.0 0.0 0.0) _asbp_player))))))

(event `self.ReceiveHit`
  (params (MyComp :type "PrimitiveComponent Object Reference") (Other :type "Actor Object Reference") (OtherComp :type "PrimitiveComponent Object Reference") (bSelfMoved :type Boolean) (HitLocation :type "Vector Structure") (HitNormal :type "Vector Structure") (NormalImpulse :type "Vector Structure") (Hit :type "HitResult Structure (by ref)"))
  (bind _asbp_player (cast `/Game/Blueprints/BP_Player` Other))
  (`/Game/Blueprints/BP_Player.Hit` _asbp_player (`SceneComponent.K2_GetComponentLocation` (`self.CapsuleComponent`)) (`self.KnockbackDamage`))
  (`self.DestroyEnemy`))

(fn `CheckDirState`
  (params (`X Axis` :type "Float (double-precision)") (`Y Axis` :type "Float (double-precision)"))
  (returns (ReturnValue :type "/Game/Enums_Structs/E_DirectionState Enum"))
  (return (select `bool` (< `Y Axis` 0.0) :`false` (select `bool` (> `Y Axis` 0.0) :`false` (select `bool` (> `X Axis` 0.0) :`false` "NewEnumerator2" :`true` "NewEnumerator3" :!type "/Game/Enums_Structs/E_DirectionState Enum") :`true` "NewEnumerator1") :`true` "NewEnumerator0")))

(fn `DestroyEnemy`
  (`GameplayStatics.SpawnEmitterAtLocation` "/Game/InfinityBladeEffects/Effects/FX_Monsters/FX_Monster_Gruntling/Bomber/P_BomberExplode.P_BomberExplode" (`SceneComponent.K2_GetComponentLocation` (`self.GroundPoint`)) (struct) (0.7 0.7 0.7))
  (`GameplayStatics.PlayWorldCameraShake` "/Game/Blueprints/BP_EnemyDeathShake.BP_EnemyDeathShake_C" (`SceneComponent.K2_GetComponentLocation` (`self.CapsuleComponent`)) 0.0 999990.0)
  (`self.K2_DestroyActor`))

(fn `Fire`
  (if (`self.isInShootingRange`)
    (if (`self.canShoot`)
      (`|SpawnActorFromClass` "/Game/Blueprints/BP_EnemyProjectile.BP_EnemyProjectile_C" (`KismetMathLibrary.MakeTransform` (`SceneComponent.K2_GetComponentLocation` (`self.CapsuleComponent`)) (`self.AimAngle`)) "Undefined" "OverrideRootScale" null (`self.ProjectileSpeed`) (`self.KnockbackDamage`) null))))

(fn `Hit`
  (params (DmgInitLoc :type "Vector Structure") (Damage :type "Float (double-precision)") (Knockback :type "Float (double-precision)"))
  (bind _gm (`self.GM`))
  (bind _gm_2 (`self.GM`))
  (bind (_returnvalue_x _returnvalue_y) (`KismetMathLibrary.BreakVector` (* (- DmgInitLoc (`SceneComponent.K2_GetComponentLocation` (`self.CapsuleComponent`))) (* -1.0 Knockback))))
  (set `self.Health` (- (`self.Health`) Damage))
  (`self.LaunchCharacter` (`KismetMathLibrary.MakeVector` _returnvalue_x _returnvalue_y))
  (if (<= (`self.Health`) 0.0)
    (set `/Game/Blueprints/BP_GameModeBase.Score` (+ (`/Game/Blueprints/BP_GameModeBase.Score` _gm_2) (`self.ScoreOnKill`)) _gm_2)
    (set `/Game/Blueprints/BP_GameModeBase.Coins` (+ (`/Game/Blueprints/BP_GameModeBase.Coins` _gm) (`self.CoinOnKill`)) _gm)
    (`self.DestroyEnemy`)))

(fn `SetSprite`
  (bind _walkanimations (`self.WalkAnimations`))
  (bind _idleanimations (`self.IdleAnimations`))
  (bind _returnvalue (not (`self.isPlayerInRange`)))
  (bind _returnvalue_2 (select `bool` (`self.isStrafing`) :`false` (`self.DirAnimState`) :`true` (`self.StrafingDirState`)))
  (bind (_returnvalue_x _returnvalue_y) (`KismetMathLibrary.BreakVector2D` (select `bool` (`self.isStrafing`) :`false` (`self.DirectionVector`) :`true` (`self.AimDir Vector`))))
  (bind _returnvalue_3 (`self.CheckDirState` _returnvalue_x _returnvalue_y))
  (if (`self.isStrafing`)
    (set `self.StrafingDirState` _returnvalue_3)
    (elif _returnvalue
      (set `self.DirAnimState` _returnvalue_3)))
  (`PaperFlipbookComponent.SetFlipbook` (`self.Sprite`) (select `bool` _returnvalue :`false` (select `/Game/Enums_Structs/E_DirectionState` _returnvalue_2 :`NewEnumerator0` (`|GetArrayItem` _idleanimations) :`NewEnumerator1` (`|GetArrayItem` _idleanimations 1) :`NewEnumerator2` (`|GetArrayItem` _idleanimations 2) :`NewEnumerator3` (`|GetArrayItem` _idleanimations 3)) :`true` (select `/Game/Enums_Structs/E_DirectionState` _returnvalue_2 :`NewEnumerator0` (`|GetArrayItem` _walkanimations) :`NewEnumerator1` (`|GetArrayItem` _walkanimations 1) :`NewEnumerator2` (`|GetArrayItem` _walkanimations 2) :`NewEnumerator3` (`|GetArrayItem` _walkanimations 3)))))

(fn `SpawnCoins`)

(fn `UserConstructionScript`)